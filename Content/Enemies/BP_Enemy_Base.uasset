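; Base enemy character that supplies shared behavior for kneeling, surrendering, patrolling and movement speed.
; Kneeling and Surrendering events play montages and call their end notifications on completion or interruption, with kneeling also setting IsKneeling.
; Functions expose fixed attack and defend radii and the patrol route, and map a speed state to max walk speed.
; BeginPlay and AnyDamage are empty, and SetMovementSpeed always returns zero.
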(event `self.ReceiveBeginPlay`)

(event `Kneeling`
  (`|PlayMontage` (`self.Mesh`) "/Game/Animations/Surrendering/Montage_Kneeling.Montage_Kneeling"
    (:`OnCompleted`
      _)
    (:`OnInterrupted`
      _))
  (set `self.IsKneeling` true)
  (`self.OnKneelingEnd`))

(event `Surrendering`
  (`|PlayMontage` (`self.Mesh`) "/Game/Animations/Surrendering/Montage_Surrendering.Montage_Surrendering"
    (:`OnCompleted`
      _)
    (:`OnInterrupted`
      _))
  (`self.OnSurrenderingEnd`))

(event `self.ReceiveAnyDamage`
  (params (Damage :type "Float (single-precision)") (DamageType :type "DamageType Object Reference") (InstigatedBy :type "Controller Object Reference") (DamageCauser :type "Actor Object Reference")))

(fn `GetIdealRange`
  (returns (AttackRadius :type "Float (double-precision)") (DefendRadius :type "Float (double-precision)"))
  (return 150.0 350.0))

(fn `GetPatrolRoute`
  (returns (PatrolRoute :type "/Game/Enemies/AI/BP_PatrolRoute Object Reference"))
  (return (`self.PatrolRoute`)))

(fn `SetMovementSpeed`
  (params (Speed :type "/Game/Enemies/AI/Enums/E_MovementSpeed Enum" :default "NewEnumerator0"))
  (returns (SpeedValue :type "Float (double-precision)"))
  (set `CharacterMovementComponent.MaxWalkSpeed` (select `/Game/Enemies/AI/Enums/E_MovementSpeed` Speed :`NewEnumerator1` 100.0 :`NewEnumerator2` 300.0 :`NewEnumerator3` 500.0 :!type "Float (single-precision)") (`self.CharacterMovement`))
  (return 0.0))

(fn `UserConstructionScript`)