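; BP_Enemy_Melee is a sword-wielding enemy that implements attack, equip and unequip weapon events.
; Each event plays a montage (slash, draw or fold) and calls a dispatcher to report back, with attack end also firing on interruption.
; Montage notifies time the weapon swap: drawing spawns BP_Weapon_Sword on the right-hand socket, folding destroys it, and both update IsWieldingWeapon.
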(event `/Game/Enemies/AI/BPI_EnemyIA.Attack`
  (`|PlayMontage` (`self.Mesh`) "/Game/Animations/Sword/Montage_Sword_Slash.Montage_Sword_Slash"
    (:`OnCompleted`
      _)
    (:`OnInterrupted`
      _))
  (`self.OnAttackEnd`))

(event `/Game/Enemies/AI/BPI_EnemyIA.EquipWeapon`
  (bind _notifyname (`|PlayMontage` (`self.Mesh`) "/Game/Animations/Sword/Montage_SwordDraw.Montage_SwordDraw")
    (:`OnCompleted`
      (`self.OnWeaponEquipped`))
    (:`OnNotifyBegin`
      (switch `name` _notifyname
        (:`GrabSword`
          (bind _returnvalue (`|SpawnActorFromClass` "/Game/Weapons/BP_Weapon_Sword.BP_Weapon_Sword_C" (`self.GetTransform`) "Undefined" "OverrideRootScale" null null))
          (bind _output_get (set `self.WeaponActor` _returnvalue))
          (`self.K2_AttachToComponent` _output_get (`self.Mesh`) "hand_r_sword_socket" "SnapToTarget" "SnapToTarget" "SnapToTarget" true)
          (set `self.IsWieldingWeapon` true))))))

(event `/Game/Enemies/AI/BPI_EnemyIA.UnequipWeapon`
  (bind _notifyname (`|PlayMontage` (`self.Mesh`) "/Game/Animations/Sword/Montage_SwordFold.Montage_SwordFold")
    (:`OnCompleted`
      (`self.OnWeaponUnequipped`))
    (:`OnNotifyBegin`
      (switch `name` _notifyname
        (:`DropSword`
          (`self.K2_DestroyActor` (`self.WeaponActor`))
          (set `self.IsWieldingWeapon` false))))))

(fn `UserConstructionScript`
  (`parent.UserConstructionScript`))